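; Player controller for a tile-based building game, handling UI screens, camera, building placement and water level.
; A state enum switches widget visibility, while input pans, spins and zooms the BP_CameraFocus pawn.
; Spawned buildings attach to the clicked tile; Tick projects the cursor onto Z=0 but transforms the controller, not the building.
; It spawns a water plane raised by the Water rate; deletion mode sets a flag, but its removal logic is unwired.
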(event `self.ReceiveBeginPlay`
  (`self.SetCurrentState` "NewEnumerator0")
  ;[1 1 1] Add WaterPlane to world
  (bind _returnvalue (`|SpawnActorFromClass` "/Game/BP_WaterPlane.BP_WaterPlane_C" (`KismetMathLibrary.MakeTransform` (0.0 0.0 -360.0)) "Undefined" "OverrideRootScale" null null))
  (set `self.WaterLevelRef` _returnvalue)
  (set `self.WaterLevel` -360.0))

(event `SetCurrentState`
  (params (StateToSetToo :type "/Game/BP_Controllers/ENUM_GameState Enum" :default "NewEnumerator0"))
  ;[1 1 1] Set the current game state
  (set `self.CurrentState` StateToSetToo)
  ;[1 1 1] Check what the game state is
  (`|ExecutionSequence`
    (:`then_0`
      ;[1 1 1] Add all widgets to the player's viewport and place them in the array.
      (if (`|EnumEquality` "NewEnumerator0" (`self.CurrentState`))
        (bind _returnvalue (`|CreateWidget` "/Game/User_Interface/StartScreen/WBP_SSMain.WBP_SSMain_C"))
        (bind _output_get (set `self.StartWidget` _returnvalue))
        (set `/Game/User_Interface/StartScreen/WBP_SSMain.PlayerRef` self _output_get)
        (`UserWidget.AddToViewport` _output_get 0)
        (`KismetArrayLibrary.Array_Add` (`self.WidgetArray`) _output_get)
        (bind _returnvalue_2 (`|CreateWidget` "/Game/User_Interface/InGame/WBP_IGMain.WBP_IGMain_C"))
        (bind _output_get_2 (set `self.InGameWidget` _returnvalue_2))
        (`UserWidget.AddToViewport` _output_get_2 0)
        (`KismetArrayLibrary.Array_Add` (`self.WidgetArray`) _output_get_2)
        (set `/Game/User_Interface/InGame/WBP_IGMain.PlayerRef` self _output_get_2)
        (bind _returnvalue_3 (`|CreateWidget` "/Game/User_Interface/InGame/WBP_BuyMenu.WBP_BuyMenu_C"))
        (bind _output_get_3 (set `self.BuyMenuWidget` _returnvalue_3))
        (`UserWidget.AddToViewport` _output_get_3 0)
        (`KismetArrayLibrary.Array_Add` (`self.WidgetArray`) _output_get_3)
        (set `/Game/User_Interface/InGame/WBP_BuyMenu.PlayerRef` self _output_get_3)
        (`self.SetCurrentState` "NewEnumerator1")))
    (:`then_1`
      ;[1 1 1] Hid all widgets, then un-hide the Start Screen Widget
      (if (`|EnumEquality` "NewEnumerator1" (`self.CurrentState`))
        (for _array_element (`self.WidgetArray`)
          (if (== _array_element (`self.StartWidget`))
            (`Widget.SetVisibility` _array_element "Visible")
            (else
              (`Widget.SetVisibility` _array_element "Hidden"))))))
    (:`then_2`
      ;[1 1 1] Hide all widgets, then un-hide the In-Game Widget
      (if (`|EnumEquality` "NewEnumerator2" (`self.CurrentState`))
        (for _array_element_2 (`self.WidgetArray`)
          (if (== _array_element_2 (`self.InGameWidget`))
            (`Widget.SetVisibility` _array_element_2 "Visible")
            (else
              (`Widget.SetVisibility` _array_element_2 "Hidden"))))))))

(event `ToggleMenuState`
  (params (`MakeVisible?` :type Boolean))
  (bind _buymenuwidget (`self.BuyMenuWidget`))
  ;[1 1 1] Makes the Menu Visible Based on the input
  (if `MakeVisible?`
    (`Widget.SetVisibility` _buymenuwidget "Visible")
    (else
      (`Widget.SetVisibility` _buymenuwidget "Hidden"))))

(event `InputAction|CameraRotate`
  (params (Key :type "Key Structure"))
  (:`Pressed`
    (set `self.IsRotating` true))
  (:`Released`
    (set `self.IsRotating` false)))

(event `SetBuildingToBePlaced`
  (params (BuildingData :type "BuildingData Structure"))
  ;[1 1 1] Spawns a building to attach to a tile
  (bind _returnvalue (`|SpawnActorFromClass` "/Script/ClimateChangeGame.Building" (`KismetMathLibrary.MakeTransform` (0.0 0.0 0.0)) "AlwaysSpawn" "OverrideRootScale" null null))
  (set `self.BuildingToAttach` _returnvalue))

(event `InputAxis|MoveX`
  (params (AxisValue :type "Float (single-precision)"))
  (`self.MoveCameraBy` (`KismetMathLibrary.MakeVector` AxisValue)))

(event `InputAxis|MoveY`
  (params (AxisValue :type "Float (single-precision)"))
  (`self.MoveCameraBy` (`KismetMathLibrary.MakeVector` 0.0 AxisValue)))

(event `IncreaseWaterHeight`
  ;[1 1 1] Allows the water height to be increased
  (bind _output_get (set `self.WaterLevel` (+ (`BlueprintMapLibrary.Map_Find` (`self.Rates`) "VE_Water") -360.0)))
  (`/Game/BP_WaterPlane.UpdateWaterPos` (`self.WaterLevelRef`) _output_get))

(event `SetDelectionMode`
  (params (`CanDelete?` :type Boolean))
  ;[1 1 1] Set if deletion mode is on or not
  (set `self.RemoveBuilding?` `CanDelete?`))

(event `MoveCameraBy`
  (params (IncrementBy :type "Vector Structure"))
  (bind _returnvalue (`self.K2_GetPawn`))
  (if (not (`KismetMathLibrary.Vector_IsNearlyZero` IncrementBy))
    (bind _asbp_camera_focus (cast `/Game/BP_CameraFocus` _returnvalue))
    (set `self.FocusLocation` (+ (`KismetMathLibrary.GreaterGreater_VectorRotator` (* (* IncrementBy (`SpringArmComponent.TargetArmLength` (`/Game/BP_CameraFocus.SpringArm` _asbp_camera_focus))) 0.005) (`KismetMathLibrary.ComposeRotators` (`self.K2_GetActorRotation` _returnvalue) (struct :`Yaw` 90.0))) (`self.FocusLocation`)))
    (`self.UpdateCamera`)))

(event `self.ReceiveTick`
  (params (DeltaSeconds :type "Float (single-precision)"))
  (bind (_worldlocation _worlddirection) (`self.DeprojectMousePositionToWorld`))
  ;[1 1 1] Attach Building object to mouse, and update its position every tick
  (if (`KismetSystemLibrary.IsValid` (`self.BuildingToAttach`))
    (`self.K2_SetActorTransform` (`KismetMathLibrary.MakeTransform` (+ _worldlocation (* (* _worlddirection (/ (.z _worldlocation) (.z _worlddirection))) -1.0))))))

(event `InputAxis|MouseX`
  (params (AxisValue :type "Float (single-precision)"))
  (if (not (`KismetMathLibrary.NearlyEqual_FloatFloat` AxisValue))
    (`self.SpinCameraBy` (* AxisValue 10.0))))

(event `InputAction|Select`
  (params (Key :type "Key Structure"))
  (:`Pressed`
    ;[1 1 1] Gives tile clicked on
    (bind _tilecoordinate (`self.GetTileCoordinateCurrentlyHovered`))
    (bind _returnvalue (`GridLibrary.TileIndexToWorldPosition` _tilecoordinate))
    (`KismetSystemLibrary.PrintString` (`KismetStringLibrary.Conv_VectorToString` _returnvalue))
    ;[1 1 1] Check if there is a building to attach
    (if (`KismetSystemLibrary.IsValid` (`self.BuildingToAttach`))
      ;[1 1 1] Attach Building to tile selected
      (bind _returnvalue_2 (`Building.AttachToPosition` (`self.BuildingToAttach`) _tilecoordinate))
      (`KismetSystemLibrary.PrintString` (`KismetStringLibrary.Conv_BoolToString` _returnvalue_2))
      (set `self.BuildingToAttach` null)
      (else
        ;[1 1 1] Check if DeletionMode is true
        (if (`self.RemoveBuilding?`)
          _)))))

(event `SpinCameraBy`
  (params (`Increment By` :type "Float (double-precision)"))
  (if (`self.IsRotating`)
    (set `self.FocusRotation` (+ `Increment By` (`self.FocusRotation`)))
    (`self.UpdateCamera`)))

(event `InputAxis|Zoom`
  (params (AxisValue :type "Float (single-precision)"))
  (if (not (`KismetMathLibrary.NearlyEqual_FloatFloat` AxisValue))
    (bind _asbp_camera_focus (cast `/Game/BP_CameraFocus` (`self.K2_GetPawn`)))
    (bind _springarm (`/Game/BP_CameraFocus.SpringArm` _asbp_camera_focus))
    (set `SpringArmComponent.TargetArmLength` (+ (`SpringArmComponent.TargetArmLength` _springarm) (* AxisValue 200.0)) _springarm)))

(event `UpdateCamera`
  (`self.K2_SetActorLocationAndRotation` (`self.K2_GetPawn`) (`self.FocusLocation`) (`KismetMathLibrary.MakeRotator` 0.0 0.0 (`self.FocusRotation`)) false false))

(fn `UserConstructionScript`)
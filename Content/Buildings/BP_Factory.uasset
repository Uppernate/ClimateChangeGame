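; BP_Factory is a building Blueprint that scatters randomized instanced mesh variants within a small circle around its local origin.
; On each OnNewInstance event, it derives a distribution from the index and instance data, then generates a random variant, rotation and scale.
; It replaces the location with a random-angle, square-root-weighted radius for uniform disc coverage, then adds the instance to that variant.
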(event `self.OnNewInstance`
  (params (Index :type Integer) (Data :type "BuildingData Structure"))
  (bind (_variations _rates _instancecount _distributionrandomness) (break `BuildingData` Data))
  (bind (_variant _returnvalue) (`self.GenerateRandomVariantAndTransform` Data (`BuildingLibrary.GenerateRandomDistribution` Index _instancecount _distributionrandomness)))
  (`self.AddInstanceTo` _variant (`KismetMathLibrary.MakeTransform` (* (`KismetMathLibrary.GetForwardVector` (`KismetMathLibrary.RotatorFromAxisAndAngle` (0.0 0.0 1.0) (`KismetMathLibrary.RandomFloatInRange` 0.0 360.0))) (* (`KismetMathLibrary.Sqrt` (`KismetMathLibrary.RandomFloatInRange` 0.0 1.0)) 80.0)) (.rotation _returnvalue) (.scale _returnvalue))))

(fn `UserConstructionScript`)
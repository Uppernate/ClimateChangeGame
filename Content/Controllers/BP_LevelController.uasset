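; BP_LevelController is a controller that drives a pan, rotate and zoom camera by moving its controlled BP_CameraFocus pawn.
; Move axes shift a stored focus location relative to pawn rotation, scaled by spring arm length so panning speeds up when zoomed out.
; Mouse X changes yaw while CameraRotate is held, and both pan and spin apply through UpdateCamera.
; Zoom adjusts the spring arm length directly, without clamping.
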(event `InputAction|CameraRotate`
  (params (Key :type "Key Structure"))
  (:`Pressed`
    (set `self.IsRotating` true))
  (:`Released`
    (set `self.IsRotating` false)))

(event `self.ReceiveTick`
  (params (DeltaSeconds :type "Float (single-precision)")))

(event `InputAxis|MoveX`
  (params (AxisValue :type "Float (single-precision)"))
  (`self.MoveCameraBy` (`KismetMathLibrary.MakeVector` AxisValue)))

(event `InputAxis|MoveY`
  (params (AxisValue :type "Float (single-precision)"))
  (`self.MoveCameraBy` (`KismetMathLibrary.MakeVector` 0.0 AxisValue)))

(event `MoveCameraBy`
  (params (IncrementBy :type "Vector Structure"))
  (bind _returnvalue (`self.K2_GetPawn`))
  (if (not (`KismetMathLibrary.Vector_IsNearlyZero` IncrementBy))
    (bind _asbp_camera_focus (cast `/Game/BP_CameraFocus` _returnvalue))
    (set `self.FocusLocation` (+ (`KismetMathLibrary.GreaterGreater_VectorRotator` (* (* IncrementBy (`SpringArmComponent.TargetArmLength` (`/Game/BP_CameraFocus.SpringArm` _asbp_camera_focus))) 0.005) (`KismetMathLibrary.ComposeRotators` (`self.K2_GetActorRotation` _returnvalue) (struct :`Yaw` 90.0))) (`self.FocusLocation`)))
    (`self.UpdateCamera`)))

(event `InputAxis|MouseX`
  (params (AxisValue :type "Float (single-precision)"))
  (if (not (`KismetMathLibrary.NearlyEqual_FloatFloat` AxisValue))
    (`self.SpinCameraBy` (* AxisValue 10.0))))

(event `SpinCameraBy`
  (params (`Increment By` :type "Float (double-precision)"))
  (if (`self.IsRotating`)
    (set `self.FocusRotation` (+ `Increment By` (`self.FocusRotation`)))
    (`self.UpdateCamera`)))

(event `InputAxis|Zoom`
  (params (AxisValue :type "Float (single-precision)"))
  (if (not (`KismetMathLibrary.NearlyEqual_FloatFloat` AxisValue))
    (bind _asbp_camera_focus (cast `/Game/BP_CameraFocus` (`self.K2_GetPawn`)))
    (bind _springarm (`/Game/BP_CameraFocus.SpringArm` _asbp_camera_focus))
    (set `SpringArmComponent.TargetArmLength` (+ (`SpringArmComponent.TargetArmLength` _springarm) (* AxisValue 200.0)) _springarm)))

(event `UpdateCamera`
  (`self.K2_SetActorLocationAndRotation` (`self.K2_GetPawn`) (`self.FocusLocation`) (`KismetMathLibrary.MakeRotator` 0.0 0.0 (`self.FocusRotation`)) false false))

(fn `UserConstructionScript`)